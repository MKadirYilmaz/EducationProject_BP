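; Player actor for a missile survival game, with control-rotation movement, mouse look and a cooldown dash that moves without sweep.
; A self-rescheduling timer spawns missiles in random directions around the player at shrinking, clamped intervals.
; Tick regenerates health, feeds it to the PlayerUI widget and increments its score by time survived.
; Depleted health or hitting anything not tagged Missile calls GameOver, which removes the UI and destroys the actor.
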(event OnComponentHit(PlayerMesh)
  (params (HitComponent :type Primitive%20Component%20Object%20Reference) (OtherActor :type Actor%20Object%20Reference) (OtherComp :type Primitive%20Component%20Object%20Reference) (NormalImpulse :type Vector :default "0, 0, 0") (Hit :type Hit%20Result%20Structure%20%28by%20ref%29))
  (if (not (Actor|ActorHasTag OtherActor "Missile"))
    (CallFunction|GameOver) ; If player hit something other than missile, end the game
  ))

(event Custom|SpawnMissile
  (Game|SpawnActorfromClass "/Game/Blueprint/Missile.Missile_C" (Math|Transform|MakeTransform (+ (Transformation|GetActorLocation) (* (Math|Random|RandomUnitVector) (Variables|Default|GetMissileSpawnDistance)))) "Undefined" "MultiplyWithRoot" 0 0)
  (Development|PrintString "MissileSpawned" true false "(R=0.000000,G=0.660000,B=1.000000,A=1.000000)" 0.5)
  (Variables|Default|SetMissileSpawnRate (Math|Float|Clamp(Float) (- (Variables|Default|GetMissileSpawnRate) (* (Variables|Default|GetMissileSpawnRate) 0.1)) 0.25 1e+01))
  (Development|PrintString (Utilities|String|ToString(Float) (Math|Float|Clamp(Float) (- (Variables|Default|GetMissileSpawnRate) (* (Variables|Default|GetMissileSpawnRate) 0.1)) 0.25 1e+01)) true false "(R=0.805187,G=0.000000,B=1.000000,A=1.000000)" 1.0)
  (Utilities|Time|SetTimerbyEvent (delegate Custom|SpawnMissile) (Variables|Default|GetMissileSpawnRate)))

(event Custom|ResetCanDash
  (Variables|Default|SetCanDash true)
  (Development|PrintString "You can dash now" true false "(R=1.000000,G=0.000000,B=0.936230,A=1.000000)"))

(event EventBeginPlay
  (Utilities|Time|SetTimerbyEvent (delegate Custom|SpawnMissile) (Variables|Default|GetMissileSpawnRate))
  (bind _returnvalue (UserInterface|CreateWidget "/Game/Blueprint/PlayerUI.PlayerUI_C" (Game|GetPlayerController 0)))
  (bind _output_get (Variables|Default|SetUI _returnvalue))
  (UserInterface|Viewport|AddtoViewport _output_get 0))

(event EventTick
  (params (DeltaSeconds :type Float%20%28single-precision%29))
  (bind _ui (Variables|Default|GetUI))
  (bind _output_get (Variables|Default|SetPlayerHealth (Math|Float|Clamp(Float) (+ (* DeltaSeconds (Variables|Default|GetHealthRegenSpeed)) (Variables|Default|GetPlayerHealth)) 0.0 1e+02)))
  (Variables|/Game/Blueprint/PlayerUI.PlayerUI_C|SetPlayerHealth _ui _output_get)
  (Variables|/Game/Blueprint/PlayerUI.PlayerUI_C|SetPlayerScore _ui (+ (Variables|/Game/Blueprint/PlayerUI.PlayerUI_C|GetPlayerScore _ui) DeltaSeconds)))

(event Game|Damage|EventAnyDamage
  (params (Damage :type Float%20%28single-precision%29) (DamageType :type Damage%20Type%20Object%20Reference) (InstigatedBy :type Controller%20Object%20Reference) (DamageCauser :type Actor%20Object%20Reference))
  (Development|PrintString (Utilities|String|Append (Utilities|String|ToString(Float) Damage) " damage applied by" (Utilities|GetDisplayName DamageCauser)) true false "(R=1.000000,G=0.683264,B=0.000000,A=1.000000)")
  (bind _output_get (Variables|Default|SetPlayerHealth (- (Variables|Default|GetPlayerHealth) Damage)))
  (if (<= _output_get 0.0)
    (CallFunction|GameOver)))

(event Input|ActionEvents|InputActionDash
  (params (Key :type Key%20Structure :default "None"))
  (:Pressed
    (if (Variables|Default|GetCanDash)
      (Transformation|AddActorWorldOffset (select (and (== (Variables|Default|GetForwardAxisValue) 0.0) (== (Variables|Default|GetRightAxisValue) 0.0)) (* (Math|Vector|GetForwardVector (Pawn|GetControlRotation :!class /Script/Engine.Pawn)) (Variables|Default|GetDashDistance)) (* (Math|Vector|Normalize (+ (* (Math|Vector|GetForwardVector (Pawn|GetControlRotation :!class /Script/Engine.Pawn)) (Variables|Default|GetForwardAxisValue)) (* (Math|Vector|GetRightVector (Pawn|GetControlRotation :!class /Script/Engine.Pawn)) (Variables|Default|GetRightAxisValue)))) (Variables|Default|GetDashDistance))))
      (Variables|Default|SetCanDash false)
      (Utilities|Time|SetTimerbyEvent (delegate Custom|ResetCanDash) 2.0)
      (else
        (Development|PrintString "You can't dash" true false "(R=1.000000,G=0.079997,B=0.000000,A=1.000000)")))))

(event Input|AxisEvents|InputAxisMoveForward
  (params (AxisValue :type Float%20%28single-precision%29))
  (Variables|Default|SetForwardAxisValue AxisValue)
  (Transformation|AddActorWorldOffset (* (Math|Vector|GetForwardVector (Pawn|GetControlRotation :!class /Script/Engine.Pawn)) (Variables|Default|GetSpeed) AxisValue (Utilities|Time|GetWorldDeltaSeconds)) true))

(event Input|AxisEvents|InputAxisMoveRight
  (params (AxisValue :type Float%20%28single-precision%29))
  (Variables|Default|SetRightAxisValue AxisValue)
  (Transformation|AddActorWorldOffset (* (Math|Vector|GetRightVector (Pawn|GetControlRotation :!class /Script/Engine.Pawn)) (Variables|Default|GetSpeed) AxisValue (Utilities|Time|GetWorldDeltaSeconds)) true))

(event Input|AxisEvents|InputAxisLookUp
  (params (AxisValue :type Float%20%28single-precision%29))
  (Pawn|Input|AddControllerPitchInput (* AxisValue (Variables|Default|GetMouseSensitivity) (Utilities|Time|GetWorldDeltaSeconds))))

(event Input|AxisEvents|InputAxisLookRight
  (params (AxisValue :type Float%20%28single-precision%29))
  (Pawn|Input|AddControllerYawInput (* AxisValue (Variables|Default|GetMouseSensitivity) (Utilities|Time|GetWorldDeltaSeconds))))

(fn ConstructionScript)

(fn GameOver
  (Widget|RemovefromParent (Variables|Default|GetUI))
  (Actor|DestroyActor))