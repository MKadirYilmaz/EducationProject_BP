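; Homing missile actor that chases the first player's pawn and damages whatever blocks it.
; Each Tick it turns smoothly and moves toward the player until CheckDistance triggers boost, which locks it onto a straight forward path and starts a self-destruct timer.
; Swept per-frame offsets, not scaled by delta time, feed hit results to Explode, which applies damage and destroys the missile.
; It also destroys itself when no player pawn exists.
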(event EventBeginPlay)

(event Collision|EventActorBeginOverlap
  (params (OtherActor :type Actor%20Object%20Reference)))

(event EventTick
  (params (DeltaSeconds :type Float%20%28single-precision%29))
  (bind _missilemesh (Variables|Default|GetMissileMesh))
  (Utilities|IsValid (Game|Player|GetPlayerPawn 0)
    (:Is%20Valid
      (if (Variables|Default|GetIsBoostActive)
        (bind _sweephitresult (Transformation|AddWorldOffset _missilemesh (* (Math|Vector|GetForwardVector _missilemesh) (Variables|Default|GetMissileSpeedBoosted)) true false))
        (CallFunction|Explode _sweephitresult)
        (else
          (CallFunction|CheckDistance)
          (Transformation|SetWorldRotation (Variables|Default|GetMissileMesh) (Math|Interpolation|RInterpTo (Transformation|GetWorldRotation (Variables|Default|GetMissileMesh)) (Math|Rotator|FindLookatRotation (Transformation|GetWorldLocation (Variables|Default|GetMissileMesh)) (Transformation|GetActorLocation (Game|Player|GetPlayerPawn 0))) DeltaSeconds 5.0) false false)
          (bind _output_get (Variables|Default|SetDirectionVector (Math|Vector|Normalize (- (Transformation|GetActorLocation (Game|Player|GetPlayerPawn 0)) (Transformation|GetWorldLocation (Variables|Default|GetMissileMesh))))))
          (bind _sweephitresult_2 (Transformation|AddWorldOffset (Variables|Default|GetMissileMesh) (* _output_get (Variables|Default|GetMissileSpeed)) true false))
          (CallFunction|Explode _sweephitresult_2))))
    (:Is%20Not%20Valid
      (Actor|DestroyActor))))

(fn ConstructionScript)

(fn CheckDistance
  (if (< (Math|Vector|Distance(Vector) (Transformation|GetWorldLocation (Variables|Default|GetMissileMesh)) (Transformation|GetActorLocation (Game|Player|GetPlayerPawn 0))) (Variables|Default|GetMissileBoostDistance))
    (Variables|Default|SetIsBoostActive true)
    (Utilities|Time|SetTimerbyFunctionName 0 "TimeoutMissile" 5.0) ; After enabling boost, missile has maximum 5 seconds of lifetime
  ))

(fn TimeoutMissile
  (Development|PrintString (Utilities|String|Append (Utilities|GetDisplayName self) " missile time out...") true true "(R=1.000000,G=0.000000,B=0.000000,A=1.000000)")
  (Actor|DestroyActor))

(fn Explode
  (params (Hit :type Hit%20Result%20Structure%20%28by%20ref%29))
  (bind (_bblockinghit _binitialoverlap _time _distance _location _impactpoint _normal _impactnormal _physmat _hitactor) (Collision|BreakHitResult Hit))
  (if _bblockinghit
    (Game|Damage|ApplyDamage _hitactor (Variables|Default|GetMissileDamage) (Game|GetInstigatorController (Game|Player|GetPlayerPawn 0)) self "/Script/Engine.DamageType")
    (Actor|DestroyActor)))